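; BP_SpawnRandom runs a timed find-the-wrong-objects task by randomly mixing correct and faulty items in the scene.
; BeginPlay randomly marks CountTrueObject slots to keep, then moves FalsePlaceObject actors onto the other slots and destroys the correct ones there.
; A Timeline drives the timer text, while externally triggered events count selections and Proverka stops it when all replaced items are correctly selected.
; The construction script sizes the arrays, clamps counts and initializes the counter texts.
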(event EventSelectTrueObject
  ;[1 1 1] Выбран ли правильный предмет
  (bind _result (Math|Integer|IncrementInt (Variables|Default|GetSelectCorrectObjectInScene))
    (:%20%20
      (Variables|Default|SetSelectCorrectObjectInScene _result))))

(event EventSelectCountObject
  ;[1 1 1] Счетчик выбранных предметов
  (bind _result (Math|Integer|IncrementInt (Variables|Default|GetSelectCountObjectInScene))
    (:%20%20
      (bind _output_get (Variables|Default|SetSelectCountObjectInScene _result))
      (Rendering|Components|TextRender|SetText (Variables|Default|Get?/*) (Utilities|Text|ToText(Integer) _output_get)))))

(event EventNotTrueObject
  ;[1 1 1] Выбран ли правильный предмет
  (bind _result (Math|Integer|DecrementInt (Variables|Default|GetSelectCorrectObjectInScene))
    (:%20%20
      (Variables|Default|SetSelectCorrectObjectInScene _result))))

(event EventBeginPlay
  ;[1 1 1] Задаем колличество правильных предметов
  (Utilities|Array|Resize (Variables|Default|GetTruePlaceObject) (Variables|Default|GetCountObject))
  ;[1 1 1] Задаем колличество неправильных предметов
  (Utilities|Array|Resize (Variables|Default|GetFalsePlaceObject) (Variables|Default|GetCountObject))
  ;[1 1 1] Маасив для отслеживания правильных предметов
  (Utilities|Array|Resize (Variables|Default|GetPointSpawnObject) (Variables|Default|GetCountObject))
  ;[1 1 1] Запускаем процедуру перебора объектов
  (for _index (range 0 (- (Variables|Default|GetCountObject) 1))
    (|Поискпредметовдлязамены))
  (|Процедуразаменыправильныхпредметовнанеправильные
    (:Complete
      (Variables|Default|SetSelectCorrectObjectInScene 0)
      (Variables|Default|SetSelectCountObjectInScene 0)
      (bind _newtrack_0 (Timeline|Timeline_0 Play)
        (:Update
          (Rendering|Components|TextRender|SetText (Variables|Default|GetTimer) (Utilities|Text|ToText(Integer) (Math|Float|Truncate _newtrack_0))))
        (:Finished
          (Rendering|Components|TextRender|SetText (Variables|Default|GetTimer) (Utilities|Text|ToText(String) "MMM XYITA")))))))

(event EventNotCountObject
  ;[1 1 1] Счетчик выбранных предметов
  (bind _result (Math|Integer|DecrementInt (Variables|Default|GetSelectCountObjectInScene))
    (:%20%20
      (bind _output_get (Variables|Default|SetSelectCountObjectInScene _result))
      (Rendering|Components|TextRender|SetText (Variables|Default|Get?/*) (Utilities|Text|ToText(Integer) _output_get)))))

(event EventProverka
  (bind _counttrueobject (Variables|Default|GetCountTrueObject))
  (bind _countobject (Variables|Default|GetCountObject))
  (bind _returnvalue (- _countobject _counttrueobject))
  (if (and (== (Variables|Default|GetSelectCorrectObjectInScene) _returnvalue) (== _returnvalue (Variables|Default|GetSelectCountObjectInScene)))
    (bind _newtrack_0 (Timeline|Timeline_0 Stop)
      (:Update
        (Rendering|Components|TextRender|SetText (Variables|Default|GetTimer) (Utilities|Text|ToText(Integer) (Math|Float|Truncate _newtrack_0))))
      (:Finished
        (Rendering|Components|TextRender|SetText (Variables|Default|GetTimer) (Utilities|Text|ToText(String) "MMM XYITA"))))))

(fn ConstructionScript
  ;[1 1 1] Задаем колличество правильных предметов
  (Utilities|Array|Resize (Variables|Default|GetTruePlaceObject) (Variables|Default|GetCountObject))
  ;[1 1 1] Задаем колличество неправильных предметов
  (Utilities|Array|Resize (Variables|Default|GetFalsePlaceObject) (Variables|Default|GetCountObject))
  ;[1 1 1] Маасив для отслеживания правильных предметов
  (Utilities|Array|Resize (Variables|Default|GetPointSpawnObject) (Variables|Default|GetCountObject))
  (if (>= (Variables|Default|GetCountObject) 0)
    _
    (else
      (Variables|Default|SetCountObject 0)))
  ;[1 1 1] Проверяем, правильно ли ввели колличество объектов
  (if (and (>= (Variables|Default|GetCountTrueObject) 0) (<= (Variables|Default|GetCountTrueObject) (Variables|Default|GetCountObject)))
    ;[1 1 1] Если все норм, запоминаем
    (Variables|Default|SetCountTrueObject (Variables|Default|GetCountTrueObject))
    (elif (< (Variables|Default|GetCountTrueObject) 0)
      ;[1 1 1] Если ввели меньше нуля, исправляем на ноль
      (Variables|Default|SetCountTrueObject 0)
      (else
        ;[1 1 1] Если больше, задаем максимальное значение
        (Variables|Default|SetCountTrueObject (Variables|Default|GetCountObject)))))
  (Rendering|Components|TextRender|SetText (Variables|Default|Get*/?) (Utilities|Text|ToText(Integer) (- (Variables|Default|GetCountObject) (Variables|Default|GetCountTrueObject))))
  (Rendering|Components|TextRender|SetText (Variables|Default|Get?/*) (Utilities|Text|ToText(Integer) 0)))